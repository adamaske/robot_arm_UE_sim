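; BP_Robot is an articulated robot arm built from a base, three links and an end effector, posed by setting joint angles.
; The construction script stores these components and the tip in M-prefixed variables, and BeginPlay enables input from the first player controller.
; MoveToPose applies five angles as relative rotations, yaw for the base and end effector and pitch for the links between, giving forward-kinematic control.
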(event EventBeginPlay
  (Input|EnableInput (Game|GetPlayerController 0)))

(event Collision|EventActorBeginOverlap
  (params (OtherActor :type Actor%20Object%20Reference)))

(event EventTick
  (params (DeltaSeconds :type Float%20%28single-precision%29)))

(fn ConstructionScript
  (Variables|Default|Setm_Base (Variables|Default|Getbase))
  (Variables|Default|Setm_Link_2 (Variables|Default|Getlink_2))
  (Variables|Default|Setm_Link_3 (Variables|Default|Getlink_3))
  (Variables|Default|Setm_Link_4 (Variables|Default|Getlink_4))
  (Variables|Default|Setm_End_Effector (Variables|Default|Getend_effector))
  (Variables|Default|Setm_End_Effector_Tip (Variables|Default|Gettip_0)))

(fn MovetoPose
  (params (theta_0 :type Float%20%28double-precision%29) (theta_1 :type Float%20%28double-precision%29) (theta_2 :type Float%20%28double-precision%29) (theta_3 :type Float%20%28double-precision%29) (theta_4 :type Float%20%28double-precision%29))
  (Transformation|SetRelativeRotation (Variables|Default|Getbase) (Math|Rotator|MakeRotator 0.0 0.0 theta_0) false false)
  (Transformation|SetRelativeRotation (Variables|Default|Getlink_2) (Math|Rotator|MakeRotator 0.0 theta_1 0.0) false false)
  (Transformation|SetRelativeRotation (Variables|Default|Getlink_3) (Math|Rotator|MakeRotator 0.0 theta_2 0.0) false false)
  (Transformation|SetRelativeRotation (Variables|Default|Getlink_4) (Math|Rotator|MakeRotator 0.0 theta_3 0.0) false false)
  (Transformation|SetRelativeRotation (Variables|Default|Getend_effector) (Math|Rotator|MakeRotator 0.0 0.0 theta_4) false false))