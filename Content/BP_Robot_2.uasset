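; BP_Robot_2 is an articulated robot arm actor with pose and stats widgets shown on screen.
; The construction script assigns base, link, end effector and tip components to M-prefixed references.
; MoveToPose applies five joint angles as relative rotations: yaw at the base and end effector, pitch at the three links.
; BeginPlay enables input and creates both widgets, and Space calls PoseRobot with an IK-mode pose.
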(event EventBeginPlay
  (Input|EnableInput (Game|GetPlayerController 0))
  (bind _returnvalue (UserInterface|CreateWidget "/Game/WB_Pose.WB_Pose_C" 0 self))
  (UserInterface|Viewport|AddtoViewport _returnvalue 0)
  (bind _returnvalue_2 (UserInterface|CreateWidget "/Game/WB_Stats.WB_Stats_C" 0 self))
  (UserInterface|Viewport|AddtoViewport _returnvalue_2 0))

(event Collision|EventActorBeginOverlap
  (params (OtherActor :type Actor%20Object%20Reference)))

(event EventTick
  (params (DeltaSeconds :type Float%20%28single-precision%29)))

(event Input|KeyboardEvents|SpaceBar
  (params (Key :type Key%20Structure :default "None"))
  (:Pressed
    (Class|Robot|PoseRobot (Utilities|Struct|MakeRobot_Pose "IK" 0.0))))

(fn ConstructionScript
  (Variables|Default|Setm_Base (Variables|Default|Getbase))
  (Variables|Default|Setm_Link_2 (Variables|Default|Getlink_2))
  (Variables|Default|Setm_Link_3 (Variables|Default|Getlink_3))
  (Variables|Default|Setm_Link_4 (Variables|Default|Getlink_4))
  (Variables|Default|Setm_End_Effector (Variables|Default|Getend_effector))
  (Variables|Default|Setm_End_Effector_Tip (Variables|Default|Gettip_0)))

(fn MovetoPose
  (params (theta_0 :type Float%20%28double-precision%29) (theta_1 :type Float%20%28double-precision%29) (theta_2 :type Float%20%28double-precision%29) (theta_3 :type Float%20%28double-precision%29) (theta_4 :type Float%20%28double-precision%29))
  (Transformation|SetRelativeRotation (Variables|Default|Getbase) (Math|Rotator|MakeRotator 0.0 0.0 theta_0) false false)
  (Transformation|SetRelativeRotation (Variables|Default|Getlink_2) (Math|Rotator|MakeRotator 0.0 theta_1 0.0) false false)
  (Transformation|SetRelativeRotation (Variables|Default|Getlink_3) (Math|Rotator|MakeRotator 0.0 theta_2 0.0) false false)
  (Transformation|SetRelativeRotation (Variables|Default|Getlink_4) (Math|Rotator|MakeRotator 0.0 theta_3 0.0) false false)
  (Transformation|SetRelativeRotation (Variables|Default|Getend_effector) (Math|Rotator|MakeRotator 0.0 0.0 theta_4) false false))